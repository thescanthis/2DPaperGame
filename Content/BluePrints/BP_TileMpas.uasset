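; Tile map actor that provides grid walkability and tile positions from a Paper2D tile map.
; On BeginPlay it builds a flat boolean grid, marking cells with a layer 1 tile as blocked; deriving rows by dividing by height assumes a square map.
; CanGo and GetTilePos share GridPosToIndex for range checks, and GetTilePos maps cells to world locations on the XZ plane, with rows descending in Z.
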(event EventBeginPlay
  (bind _rendercomponent (Variables|Default|GetRenderComponent))
  (bind _tilemap (Variables|/Script/Paper2D.PaperTileMapComponent|GetTileMap _rendercomponent))
  (Utilities|FlowControl|Sequence
    (:then_0
      (Utilities|Array|Resize (Variables|Default|GetGridMap) (* (Variables|/Script/Paper2D.PaperTileMap|GetMapWidth _tilemap) (Variables|/Script/Paper2D.PaperTileMap|GetMapHeight _tilemap)))
      (Variables|Default|SetMapWidth (Variables|/Script/Paper2D.PaperTileMap|GetMapWidth _tilemap))
      (Variables|Default|SetMapHeight (Variables|/Script/Paper2D.PaperTileMap|GetMapHeight _tilemap)))
    (:then_1
      (for (_ _array_index) (Variables|Default|GetGridMap)
        (Utilities|IsValid (.tileset (Class|PaperTileMapComponent|GetTile (Variables|Default|GetRenderComponent) (Math|Integer|%(Integer) _array_index (Variables|/Script/Paper2D.PaperTileMap|GetMapWidth _tilemap)) (/ _array_index (Variables|/Script/Paper2D.PaperTileMap|GetMapHeight _tilemap)) 1))
          (:Is%20Valid
            (Utilities|Array|SetArrayElem (Variables|Default|GetGridMap) _array_index true)))))))

(fn ConstructionScript)

(fn CanGo
  (params (GridX :type Integer) (GridY :type Integer))
  (bind (_valid _index) (CallFunction|GridPostoIndex GridX GridY))
  (if _valid
    (return (not (Utilities|Array|Get(acopy) (Variables|Default|GetGridMap) _index)))
    (else
      (return false))))

(fn GridPostoIndex
  (params (GridX :type Integer) (GridY :type Integer))
  (return (and (Math|Integer|InRange(Integer) GridX 0 (Variables|Default|GetMapWidth)) (Math|Integer|InRange(Integer) GridY 0 (Variables|Default|GetMapHeight))) (+ (* GridY (Variables|Default|GetMapWidth)) GridX)))

(fn GetTilePos
  (params (Gridx :type Integer) (Gridy :type Integer))
  (bind _valid (CallFunction|GridPostoIndex Gridx Gridy))
  (return _valid (+ (Transformation|GetActorLocation) (Math|Vector|MakeVector (* Gridx (Variables|Default|GetSize_x) 5.0) 0.0 (* Gridy (Variables|Default|GetSize_y) -5)))))